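; Actor Blueprint that moves StaticMesh2 along an ellipse in its relative YZ plane.
; BeginPlay starts a looping 0.01-second timer that calls DrawElipse.
; DrawElipse sets the mesh's relative location from degree-based sine and cosine of game time times Speed, scaled by Width and Height.
; An alternative Timeline-driven version of the same movement remains in the event graph but never runs.
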(event EventBeginPlay
  (Utilities|Time|SetTimerbyFunctionName 0 "DrawElipse" 0.01 true))

(fn ConstructionScript)

(fn DrawElipse
  (bind _returnvalue (Utilities|Time|GetGameTimeinSeconds))
  (bind _speed (Variables|Default|GetSpeed))
  (bind _returnvalue_2 (* _returnvalue _speed))
  (Transformation|SetRelativeLocation (Variables|Default|GetStaticMesh2) (Math|Vector|MakeVector 0.0 (* (Math|Trig|Sin(Degrees) _returnvalue_2) (Variables|Default|GetWidth)) (* (Math|Trig|Cos(Degrees) _returnvalue_2) (Variables|Default|GetHeight))) false))